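; BP_Player is the player character Blueprint, providing jumping and movement through Enhanced Input.
; On BeginPlay, PlayerInput casts the controller to PlayerController and adds the IMC_PlayerInput mapping context.
; The left/right and up/down actions feed movement input along fixed world X and Y axes, independent of camera or control rotation.
; The jump action calls Jump when started, with no handler for release.
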(event `self.ReceiveBeginPlay`
  (`self.PlayerInput`))

(event `EnhancedInput|/Game/BP/Player/Inputs/Actions/IA_JUMP`
  (params (ActionValue :type Boolean) (ElapsedSeconds :type "Float (double-precision)") (TriggeredSeconds :type "Float (double-precision)") (InputAction :type "InputAction Object Reference" :default "/Game/BP/Player/Inputs/Actions/IA_JUMP.IA_JUMP"))
  (:`Started`
    (`self.Jump`)))

(event `EnhancedInput|/Game/BP/Player/Inputs/Actions/IA_LEFTRIEGHT`
  (params (ActionValue :type "Float (double-precision)") (ElapsedSeconds :type "Float (double-precision)") (TriggeredSeconds :type "Float (double-precision)") (InputAction :type "InputAction Object Reference" :default "/Game/BP/Player/Inputs/Actions/IA_LEFTRIEGHT.IA_LEFTRIEGHT"))
  (:`Triggered`
    (`self.AddMovementInput` (1.0 0.0 0.0) ActionValue)))

(event `EnhancedInput|/Game/BP/Player/Inputs/Actions/IA_TOPDAWN`
  (params (ActionValue :type "Float (double-precision)") (ElapsedSeconds :type "Float (double-precision)") (TriggeredSeconds :type "Float (double-precision)") (InputAction :type "InputAction Object Reference" :default "/Game/BP/Player/Inputs/Actions/IA_TOPDAWN.IA_TOPDAWN"))
  (:`Triggered`
    (`self.AddMovementInput` (0.0 1.0 0.0) ActionValue)))

(fn `PlayerInput`
  (bind _asplayer_controller (cast `PlayerController` (`self.GetController`)))
  (`EnhancedInputSubsystemInterface.AddMappingContext` (pcsubsystem `EnhancedInputLocalPlayerSubsystem` _asplayer_controller) "/Game/BP/Player/Inputs/IMC_PlayerInput.IMC_PlayerInput" 0 (struct)))

(fn `UserConstructionScript`)