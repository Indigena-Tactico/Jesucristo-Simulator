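; BP_Player1 is a player Blueprint that moves along world axes and jumps through Enhanced Input.
; BeginPlay adds the IMC_PlayerInput mapping context to its controller.
; IA_Move feeds world X and Y movement and stores the input as Direction, while IA_JUMP triggers Jump.
; Tick flips player 0's control rotation between pitch 0 and 180 by the sign of X velocity.
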(event `self.ReceiveTick`
  (params (DeltaSeconds :type "Float (single-precision)"))
  (bind _returnvalue_x (`KismetMathLibrary.BreakVector` (`self.GetVelocity`)))
  (`/Engine/EditorBlueprintResources/StandardMacros.CompareFloat` _returnvalue_x
    (:`>`
      (`Controller.SetControlRotation` (`GameplayStatics.GetPlayerController` 0) (`KismetMathLibrary.MakeRotator` 0.0)))
    (:`<`
      (`Controller.SetControlRotation` (`GameplayStatics.GetPlayerController` 0) (`KismetMathLibrary.MakeRotator` 0.0 180.0)))))

(event `self.ReceiveBeginPlay`
  (`self.AddPlayerInput`))

(event `EnhancedInput|/Game/BP/Player/Inputs/Actions/IA_JUMP`
  (params (ActionValue :type Boolean) (ElapsedSeconds :type "Float (double-precision)") (TriggeredSeconds :type "Float (double-precision)") (InputAction :type "InputAction Object Reference" :default "/Game/BP/Player/Inputs/Actions/IA_JUMP.IA_JUMP"))
  (:`Started`
    (`self.Jump`)))

(event `EnhancedInput|/Game/BP/Player/Inputs/Actions/IA_Move`
  (params (ActionValue :type "Vector2D Structure") (ElapsedSeconds :type "Float (double-precision)") (TriggeredSeconds :type "Float (double-precision)") (InputAction :type "InputAction Object Reference" :default "/Game/BP/Player/Inputs/Actions/IA_Move.IA_Move"))
  (:`Triggered`
    (`self.AddMovementInput` (1.0 0.0 0.0) ActionValue_X)
    (`self.AddMovementInput` (0.0 1.0 0.0) ActionValue_Y)
    (set `self.Direction` (`KismetMathLibrary.MakeVector2D` ActionValue_X ActionValue_Y))))

(fn `AddPlayerInput`
  (bind _asplayer_controller (cast `PlayerController` (`self.GetController`)))
  (`EnhancedInputSubsystemInterface.AddMappingContext` (pcsubsystem `EnhancedInputLocalPlayerSubsystem` _asplayer_controller) "/Game/BP/Player/Inputs/IMC_PlayerInput.IMC_PlayerInput" 0 (struct)))

(fn `UserConstructionScript`)